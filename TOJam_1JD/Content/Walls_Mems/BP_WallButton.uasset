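; BP_WallButton is a button that triggers walls or doors whose DoorValue matches its ButtonValue.
; Its Interact event searches all BP_WallMem actors and calls OpenDoor on the matches.
; Separately, overlapping its Box enables player input and opens a gate, so pressing E sends an Interact message to matching entries in DoorArray.
; Leaving the Box disables input and closes the gate.
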(event `/Game/Walls_Mems/Interact_Interface.Interact`
  (bind _outactors (`GameplayStatics.GetAllActorsOfClass` "/Game/Walls_Mems/BP_WallMem.BP_WallMem_C"))
  (for _array_element _outactors
    (if (== (`/Game/Walls_Mems/BP_WallMem.Door_Value` _array_element) (`self.Button_Value`))
      (`/Game/Walls_Mems/BP_WallMem.OpenDoor` _array_element))))

(event `Key|E`
  (params (Key :type "Key Structure"))
  (:`Pressed`
    (`/Engine/EditorBlueprintResources/StandardMacros.Gate` true :!label _label
      (:`Exit`
        (for _array_element (`self.Door_Array`)
          (if (== (`/Game/Walls_Mems/BP_WallMem.Door_Value` _array_element) (`self.Button_Value`))
            (message `/Game/Walls_Mems/Interact_Interface.Interact` _array_element)))))))

(event `self.Box.OnComponentBeginOverlap`
  (params (OverlappedComponent :type "PrimitiveComponent Object Reference") (OtherActor :type "Actor Object Reference") (OtherComp :type "PrimitiveComponent Object Reference") (OtherBodyIndex :type Integer) (bFromSweep :type Boolean) (SweepResult :type "HitResult Structure (by ref)"))
  (`self.EnableInput` (`GameplayStatics.GetPlayerController` 0))
  (goto _label :!via `Open`))

(event `self.Box.OnComponentEndOverlap`
  (params (OverlappedComponent :type "PrimitiveComponent Object Reference") (OtherActor :type "Actor Object Reference") (OtherComp :type "PrimitiveComponent Object Reference") (OtherBodyIndex :type Integer))
  (`self.DisableInput` (`GameplayStatics.GetPlayerController` 0))
  (goto _label :!via `Close`))

(fn `UserConstructionScript`)