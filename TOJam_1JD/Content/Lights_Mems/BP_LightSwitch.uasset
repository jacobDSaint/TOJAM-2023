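; BP_LightSwitch is an interactable switch that toggles the BP_Light actors sharing its LightIndex.
; BeginPlay caches every BP_Light in LightsArray.
; The BoxLight overlap enables input and opens a gate for the E key, and end overlap reverses both.
; Each gated press also sets MemoryWall's relative location from a lerp of its world location toward Z -1000, with Alpha fixed at zero.
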(event `self.ReceiveBeginPlay`
  (bind _outactors (`GameplayStatics.GetAllActorsOfClass` "/Game/Lights_Mems/BP_Light.BP_Light_C"))
  (for _array_element _outactors
    (`KismetArrayLibrary.Array_Add` (`self.Lights_Array`) _array_element)))

(event `Key|E`
  (params (Key :type "Key Structure"))
  (:`Pressed`
    (`/Engine/EditorBlueprintResources/StandardMacros.Gate` true :!label _label
      (:`Exit`
        (`SceneComponent.K2_SetRelativeLocationAndRotation` :`self` (`self.MemoryWall`) :`NewLocation` (`KismetMathLibrary.VLerp` (`SceneComponent.K2_GetComponentLocation` (`self.MemoryWall`)) (0.0 0.0 -1000.0)))
        (for _array_element (`self.Lights_Array`)
          (if (== (`/Game/Lights_Mems/BP_Light.Light_Index` _array_element) (`self.Light_Index`))
            (message `/Game/Lights_Mems/Lights_Interface.Toggle Lights` _array_element)))))))

(event `self.BoxLight.OnComponentBeginOverlap`
  (params (OverlappedComponent :type "PrimitiveComponent Object Reference") (OtherActor :type "Actor Object Reference") (OtherComp :type "PrimitiveComponent Object Reference") (OtherBodyIndex :type Integer) (bFromSweep :type Boolean) (SweepResult :type "HitResult Structure (by ref)"))
  (`self.EnableInput` (`GameplayStatics.GetPlayerController` 0))
  (goto _label :!via `Open`))

(event `self.BoxLight.OnComponentEndOverlap`
  (params (OverlappedComponent :type "PrimitiveComponent Object Reference") (OtherActor :type "Actor Object Reference") (OtherComp :type "PrimitiveComponent Object Reference") (OtherBodyIndex :type Integer))
  (`self.DisableInput` (`GameplayStatics.GetPlayerController` 0))
  (goto _label :!via `Close`))

(fn `UserConstructionScript`)